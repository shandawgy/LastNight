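; Player character Blueprint for the Smart Locomotion system, acting as a hub that routes input to gameplay components.
; Movement, camera, parkour, ladder, swimming, combat stance and ragdoll components do the work, with state checks gating conflicting actions like leaning while climbing.
; BeginPlay registers FPS and TPS cameras and adds a demo cursor widget.
; Landing calls parkour roll, while jumping triggers camera shake directly or through a server variant.
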(event `InputAxis|MoveForward` :overrideparent false
  (params (AxisValue :type "Float (single-precision)"))
  ;[0 0 0 1 100] AXIS
  ;;[0 0 0 1 30] Axis MoveForward
  (`/Game/SmartLocomotion/Blueprints/ActorComponents/AC_Movement.Move Forward` (`self.AC_Movement`) AxisValue))

(event `InputAxis|MoveRight` :overrideparent false
  (params (AxisValue :type "Float (single-precision)"))
  ;[0 0 0 1 100] AXIS
  ;;[0 0 0 1 30] Axis MoveRight
  (`/Game/SmartLocomotion/Blueprints/ActorComponents/AC_Movement.Move Right` (`self.AC_Movement`) AxisValue))

(event `InputAction|Crouch`
  (params (Key :type "Key Structure"))
  ;[0 0 0 1 100] INPUTS
  ;;[0 0 0 1 30] Input Crouch
  (:`Pressed`
    (if (not (`/Game/SmartLocomotion/Blueprints/ActorComponents/AC_Swimming.Is Swimming` (`self.AC_Swimming`)))
      (`/Game/SmartLocomotion/Blueprints/ActorComponents/AC_Movement.Crouch` (`self.AC_Movement`)))))

(event `InputAction|Jump` :overrideparent false
  (params (Key :type "Key Structure"))
  (bind _ac_ladder (`self.AC_Ladder`))
  ;[0 0 0 1 100] INPUTS
  ;;[0 0 0 1 30] Input Jump
  (:`Pressed`
    (if (`/Game/SmartLocomotion/Blueprints/ActorComponents/AC_Ladder.Is Climbing Ladder` _ac_ladder)
      (`/Game/SmartLocomotion/Blueprints/ActorComponents/AC_Ladder.Exit Ladder from Jump Server` _ac_ladder)
      (else
        (`/Game/SmartLocomotion/Blueprints/ActorComponents/AC_Parkour.Climbing` (`self.AC_Parkour`)))))
  (:`Released`
    (`self.StopJumping`)))

(event `InputAction|Sprint`
  (params (Key :type "Key Structure"))
  (bind _ac_movement (`self.AC_Movement`))
  ;[0 0 0 1 100] INPUTS
  ;;[0 0 0 1 30] Input Sprint
  (:`Pressed`
    (`/Game/SmartLocomotion/Blueprints/ActorComponents/AC_Movement.Sprint` _ac_movement true))
  (:`Released`
    (`/Game/SmartLocomotion/Blueprints/ActorComponents/AC_Movement.Sprint` _ac_movement false)))

(event `self.ReceiveBeginPlay`
  ;[0 0 0 1 100] EVENTS
  ;;[0 0 0 1 30] Begin Play
  ;;;[0 0 0] Set All Camera
  (`/Game/SmartLocomotion/Blueprints/ActorComponents/AC_Camera.Set Camera` (`self.AC_Camera`) (`self.FPS Camera`) (`self.TPS Camera`))
  ;;;[1 0 0] Cursor Widget ( Remove this for your project )
  (bind _returnvalue (`|CreateWidget` "/Game/SmartLocomotion/Blueprints/Widget_Cursor.Widget_Cursor_C"))
  (`/Engine/EditorBlueprintResources/StandardMacros.IsValid` _returnvalue
    (:`Is Valid`
      (`UserWidget.AddToViewport` _returnvalue 0))))

(event `InputAxis|Mouse X`
  (params (AxisValue :type "Float (single-precision)"))
  ;[0 0 0 1 100] AXIS
  ;;[0 0 0 1 30] Axis Mouse X
  (`/Game/SmartLocomotion/Blueprints/ActorComponents/AC_Movement.Mouse X Axis` (`self.AC_Movement`) AxisValue))

(event `InputAxis|Mouse Y`
  (params (AxisValue :type "Float (single-precision)"))
  ;[0 0 0 1 100] AXIS
  ;;[0 0 0 1 30] Axis Mouse Y
  (`self.AddControllerPitchInput` (* AxisValue 0.5)))

(event `InputAction|Default Stance`
  (params (Key :type "Key Structure"))
  ;[0 0 0 1 100] INPUTS
  ;;[0 0 0 1 30] Input Default Stance
  (:`Pressed`
    (`/Game/SmartLocomotion/Blueprints/ActorComponents/AC_CombatStances.Start Stance` (`self.AC_CombatStances`) "NewEnumerator2" null "None")))

(event `InputAction|Sword Stance`
  (params (Key :type "Key Structure"))
  ;[0 0 0 1 100] INPUTS
  ;;[0 0 0 1 30] Input Sword Stance
  (:`Pressed`
    (`/Game/SmartLocomotion/Blueprints/ActorComponents/AC_CombatStances.Start Stance` (`self.AC_CombatStances`) "NewEnumerator1" "/Game/SmartLocomotion/Blueprints/Equipable/BP_Sword.BP_Sword_C" "sword")))

(event `self.OnLanded`
  (params (Hit :type "HitResult Structure (by ref)"))
  ;[0 0 0 1 100] EVENTS
  ;;[0 0 0 1 30] On Landed
  (`/Game/SmartLocomotion/Blueprints/ActorComponents/AC_Parkour.Roll` (`self.AC_Parkour`)))

(event `InputAction|Pistol Stance`
  (params (Key :type "Key Structure"))
  ;[0 0 0 1 100] INPUTS
  ;;[0 0 0 1 30] Input Pistol Stance
  (:`Pressed`
    (`/Game/SmartLocomotion/Blueprints/ActorComponents/AC_CombatStances.Start Stance` (`self.AC_CombatStances`) "NewEnumerator0" "/Game/SmartLocomotion/Blueprints/Equipable/BP_Pistol.BP_Pistol_C" "pistol")))

(event `self.K2_OnMovementModeChanged`
  (params (PrevMovementMode :type "EMovementMode Enum" :default "MOVE_None") (NewMovementMode :type "EMovementMode Enum" :default "MOVE_None") (PrevCustomMode :type Byte) (NewCustomMode :type Byte))
  ;[0 0 0 1 100] EVENTS
  ;;[0 0 0 1 30] On Movement Mode Changed
  (switch `EMovementMode` NewMovementMode))

(event `InputAxis|Swimming Up`
  (params (AxisValue :type "Float (single-precision)"))
  ;[0 0 0 1 100] AXIS
  ;;[0 0 0 1 30] Axis Swimming Up
  (`/Game/SmartLocomotion/Blueprints/ActorComponents/AC_Swimming.Swimming Up` (`self.AC_Swimming`) AxisValue))

(event `self.OnJumped`
  (bind _ac_camera (`self.AC_Camera`))
  ;[0 0 0 1 100] EVENTS
  ;;[0 0 0 1 30] On Jumped
  (if (and (`self.IsLocallyControlled`) (`self.HasAuthority`))
    (`/Game/SmartLocomotion/Blueprints/ActorComponents/AC_Camera.Jump Shake` _ac_camera)
    (else
      (`/Game/SmartLocomotion/Blueprints/ActorComponents/AC_Camera.Jump Shake Server` _ac_camera))))

(event `InputAction|Lean Right`
  (params (Key :type "Key Structure"))
  (bind _ac_movement (`self.AC_Movement`))
  ;[0 0 0 1 100] INPUTS
  ;;[0 0 0 1 30] Input Lean Right
  (:`Pressed`
    (if (not (`/Game/SmartLocomotion/Blueprints/ActorComponents/AC_Parkour.Is Climbing` (`self.AC_Parkour`)))
      (`/Game/SmartLocomotion/Blueprints/ActorComponents/AC_Movement.Lean Right` _ac_movement true)))
  (:`Released`
    (`/Game/SmartLocomotion/Blueprints/ActorComponents/AC_Movement.Lean Right` _ac_movement false)))

(event `InputAction|Lean Left`
  (params (Key :type "Key Structure"))
  (bind _ac_movement (`self.AC_Movement`))
  ;[0 0 0 1 100] INPUTS
  ;;[0 0 0 1 30] Input Lean Left
  (:`Pressed`
    (if (not (`/Game/SmartLocomotion/Blueprints/ActorComponents/AC_Parkour.Is Climbing` (`self.AC_Parkour`)))
      (`/Game/SmartLocomotion/Blueprints/ActorComponents/AC_Movement.Lean Left` _ac_movement true)))
  (:`Released`
    (`/Game/SmartLocomotion/Blueprints/ActorComponents/AC_Movement.Lean Left` _ac_movement false)))

(event `InputAction|Switch Camera Mode`
  (params (Key :type "Key Structure"))
  ;[0 0 0 1 100] INPUTS
  ;;[0 0 0 1 30] Input Toggle View
  (:`Pressed`
    (if (not (or (`/Game/SmartLocomotion/Blueprints/ActorComponents/AC_Ragdoll.Is Ragdolling` (`self.AC_Ragdoll`)) (`/Game/SmartLocomotion/Blueprints/ActorComponents/AC_Movement.Is Leaning` (`self.AC_Movement`))))
      (`/Game/SmartLocomotion/Blueprints/ActorComponents/AC_Camera.Toggle View Mode` (`self.AC_Camera`)))))

(event `InputAction|FreeLook`
  (params (Key :type "Key Structure"))
  (bind _ac_camera (`self.AC_Camera`))
  ;[0 0 0 1 100] INPUTS
  ;;[0 0 0 1 30] Input Free Look
  (:`Pressed`
    (`/Game/SmartLocomotion/Blueprints/ActorComponents/AC_Camera.Free Look` _ac_camera true))
  (:`Released`
    (`/Game/SmartLocomotion/Blueprints/ActorComponents/AC_Camera.Free Look` _ac_camera false)))

(event `InputAction|Ragdoll`
  (params (Key :type "Key Structure"))
  ;[0 0 0 1 100] INPUTS
  ;;[0 0 0 1 30] Input Ragdoll
  (:`Pressed`
    (`/Game/SmartLocomotion/Blueprints/ActorComponents/AC_Ragdoll.Ragdoll Check` (`self.AC_Ragdoll`))))

(event `InputAction|Switch Shoulder`
  (params (Key :type "Key Structure"))
  ;[0 0 0 1 100] INPUTS
  ;;[0 0 0 1 30] Input Switch Shoulder
  (:`Pressed`
    (`/Game/SmartLocomotion/Blueprints/ActorComponents/AC_Camera.Shoulder Switch` (`self.AC_Camera`) (`self.Spring Arm TPS`))))

(event `InputAction|Debug Arrows`
  (params (Key :type "Key Structure"))
  ;[0 0 0 1 100] INPUTS
  ;;[0 0 0 1 30] Input Debug Arrows
  (:`Pressed`
    (`/Game/SmartLocomotion/Blueprints/ActorComponents/AC_Movement.Toggle Debug Arrows` (`self.AC_Movement`) (`self.Facing Arrow `) (`self.Velocity Arrow`))))

(event `InputAction|Toggle TPS Rotation Mode`
  (params (Key :type "Key Structure"))
  ;[0 0 0 1 100] INPUTS
  ;;[0 0 0 1 30] Toggle TPS Rotation Mode
  (:`Pressed`
    (if (not (`/Game/SmartLocomotion/Blueprints/ActorComponents/AC_Ladder.Is Climbing Ladder` (`self.AC_Ladder`)))
      (`/Game/SmartLocomotion/Blueprints/ActorComponents/AC_Camera.Toggle Rotation Mode` (`self.AC_Camera`)))))

(event `InputAction|Aiming`
  (params (Key :type "Key Structure"))
  (bind _ac_combatstances (`self.AC_CombatStances`))
  ;[0 0 0 1 100] INPUTS
  ;;[0 0 0 1 30] Input Aiming
  (:`Pressed`
    (if (not (or (`/Game/SmartLocomotion/Blueprints/ActorComponents/AC_Parkour.Is Climbing` (`self.AC_Parkour`)) (`/Game/SmartLocomotion/Blueprints/ActorComponents/AC_Ladder.Is Climbing Ladder` (`self.AC_Ladder`))))
      (`/Game/SmartLocomotion/Blueprints/ActorComponents/AC_CombatStances.Aiming` _ac_combatstances true)))
  (:`Released`
    (`/Game/SmartLocomotion/Blueprints/ActorComponents/AC_CombatStances.Aiming` _ac_combatstances false)))

(event `InputAction|Slide`
  (params (Key :type "Key Structure"))
  ;[0 0 0 1 100] INPUTS
  ;;[0 0 0 1 30] Input Slide
  (:`Pressed`
    (`/Game/SmartLocomotion/Blueprints/ActorComponents/AC_Parkour.Slide` (`self.AC_Parkour`))))

(fn `UserConstructionScript`)